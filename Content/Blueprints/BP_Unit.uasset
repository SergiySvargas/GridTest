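; BP_Unit is the visual actor for a unit on a grid, displaying that unit's state as a sphere.
; Init stores the unit and picks one of two sphere materials by index.
; Update moves the actor to the unit's grid position scaled by cell size at a fixed height, briefly enlarges the sphere when it just attacked, and hides it once hit points reach zero.
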(fn `Init`
  (params (Unit :type "Unit Object Reference") (Idx :type Integer))
  (set `self.Unit` Unit)
  (`PrimitiveComponent.SetMaterial` (`self.Sphere`) 0 (select `int` (`local.Idx`) :`0` "/Game/Assets/MI_Unit0.MI_Unit0" :`1` "/Game/Assets/MI_Unit1.MI_Unit1" :!type "MaterialInterface Object Reference")))

(fn `Update`
  (params (JustAttacked :type Boolean))
  (bind _size (`/Game/Blueprints/BPFL_Constants.GetGridCellSize`))
  (bind (_returnvalue_x _returnvalue_y) (`KismetMathLibrary.BreakVector2D` (* (`BPFL_Utility.GetUnitPosition` (`self.Unit`)) (`KismetMathLibrary.MakeVector2D` _size _size))))
  (`self.K2_SetActorLocation` (`KismetMathLibrary.MakeVector` _returnvalue_x _returnvalue_y 250.0))
  (`SceneComponent.SetWorldScale3D` (`self.Sphere`) (`KismetMathLibrary.SelectVector` (7.0 7.0 7.0) (5.0 5.0 5.0) (`local.JustAttacked`)))
  (`SceneComponent.SetVisibility` (`self.Sphere`) (> (`Unit.HitPoints` (`self.Unit`)) 0) false))

(fn `UserConstructionScript`)