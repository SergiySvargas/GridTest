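; Game mode that runs a grid-based unit simulation and mirrors its state onto unit actors in the level.
; On BeginPlay it constructs and initializes a Simulation object, gathers all BP_Unit actors, then starts a looping timer at the simulation frame length.
; Each tick steps the simulation and moves the first two units to their simulated positions scaled by grid cell size, matching actors to simulation units by array index.
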(event `self.ReceiveBeginPlay`
  (bind _returnvalue (`|GenericCreateObject` "/Script/GridTest.Simulation"))
  (bind _output_get (set `self.Simulation` _returnvalue))
  (`Simulation.Init` _output_get)
  (bind _outactors (`GameplayStatics.GetAllActorsOfClass` "/Game/Blueprints/BP_Unit.BP_Unit_C"))
  (set `self.Units` _outactors)
  (`KismetSystemLibrary.K2_SetTimerDelegate` (delegate `OnSimulationTick`) (`self.SimulationFrameLength`) true))

(event `OnSimulationTick`
  (`Simulation.SimulationTick` (`self.Simulation`))
  (`self.UpdateUnit` 0)
  (`self.UpdateUnit` 1))

(fn `UpdateUnit`
  (params (idx :type Integer))
  (locals (GridCellSize :type "Float (double-precision)" :default 100.0))
  (bind _gridcellsize (`local.GridCellSize`))
  (bind (_returnvalue_x _returnvalue_y) (`KismetMathLibrary.BreakVector2D` (* (`Unit.GetBlueprintCompatiblePosition` (`Simulation.GetUnit` (`self.Simulation`) (`local.idx`))) (`KismetMathLibrary.MakeVector2D` _gridcellsize _gridcellsize))))
  (`self.K2_SetActorLocation` (`|GetArrayItem` (`self.Units`) (`local.idx`)) (`KismetMathLibrary.MakeVector` _returnvalue_x _returnvalue_y) false false))

(fn `UserConstructionScript`)